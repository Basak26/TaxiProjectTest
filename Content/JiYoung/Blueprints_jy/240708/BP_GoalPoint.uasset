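; BP_GoalPoint is a taxi drop-off destination where a passenger appears after the taxi arrives.
; When a BP_Taxi overlaps its Box, it hides the goal plane and waits a short delay.
; It then spawns a BP_Passenger offset sideways in the taxi's local space, using the taxi's current rotation, for a more natural exit.
; An older spawn relative to the goal point remains unconnected.
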(event OnComponentBeginOverlap(Box)
  (params (OverlappedComponent :type Primitive%20Component%20Object%20Reference) (OtherActor :type Actor%20Object%20Reference) (OtherComp :type Primitive%20Component%20Object%20Reference) (OtherBodyIndex :type Integer) (bFromSweep :type Boolean) (SweepResult :type Hit%20Result%20Structure%20%28by%20ref%29))
  (bind _asbp_sports_car_pawn (Utilities|Casting|CastToBP_Taxi OtherActor))
  (if true
    ;[1 1 1] 골포인트에 도착하면 골 영역 사라짐
    (Rendering|SetVisibility (Variables|Default|GetPlane_GoalPoint) false false)
    ;[1 1 1] 도착 후 n초 후 손님 하차(나타남)
    (Utilities|FlowControl|Delay 3.0)
    (Game|SpawnActorfromClass "/Game/JiYoung/Blueprints_jy/BP_Passenger.BP_Passenger_C" (Math|Transform|MakeTransform (Math|Transform|TransformLocation (Math|Transform|MakeTransform (Math|Vector|MakeVector (.x (Transformation|GetActorLocation _asbp_sports_car_pawn)) (.y (Transformation|GetActorLocation _asbp_sports_car_pawn)) (.z (Transformation|GetActorLocation _asbp_sports_car_pawn))) (Transformation|GetActorRotation _asbp_sports_car_pawn)) "0.000000,200.000000,0.000000") (Math|Transform|TransformRotation (Math|Transform|MakeTransform (Math|Vector|MakeVector (.x (Transformation|GetActorLocation _asbp_sports_car_pawn)) (.y (Transformation|GetActorLocation _asbp_sports_car_pawn)) (.z (Transformation|GetActorLocation _asbp_sports_car_pawn))) (Transformation|GetActorRotation _asbp_sports_car_pawn)) "0, 0, 0") "1.000000,1.000000,1.000000") "Undefined" "MultiplyWithRoot" 0 0)))

(fn ConstructionScript)