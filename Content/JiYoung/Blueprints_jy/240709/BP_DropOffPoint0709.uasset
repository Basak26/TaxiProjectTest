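; Taxi drop-off point that lets a passenger out when the player's taxi arrives.
; Overlapping the drop-off box with a BP_Taxi hides the DropOffPoint marker, then after a short delay reveals the existing Passenger's skeletal mesh.
; Unconnected drafts of spawning a BP_Passenger beside the point or at a rotated offset remain unused, along with a debug print.
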(event OnComponentBeginOverlap(Box_DropOff)
  (params (OverlappedComponent :type Primitive%20Component%20Object%20Reference) (OtherActor :type Actor%20Object%20Reference) (OtherComp :type Primitive%20Component%20Object%20Reference) (OtherBodyIndex :type Integer) (bFromSweep :type Boolean) (SweepResult :type Hit%20Result%20Structure%20%28by%20ref%29))
  (bind _asbp_taxi (Utilities|Casting|CastToBP_Taxi OtherActor))
  (if (Utilities|IsValid _asbp_taxi)
    ;[1 1 1] 골포인트에 도착하면 골 영역 사라짐
    (Rendering|SetVisibility (Variables|Default|GetDropOffPoint) false false)
    ;[1 1 1] 도착 후 n초 후 손님 하차(나타남)
    (Utilities|FlowControl|Delay 3.0)
    (Rendering|SetVisibility (Variables|/Game/JiYoung/Blueprints_jy/BP_Passenger.BP_Passenger_C|GetSkeletalMesh (Variables|Default|GetPassenger)) true false)))

(fn ConstructionScript)