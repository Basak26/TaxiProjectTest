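; BP_Passenger0709 is a taxi passenger actor that shows an interaction prompt when a taxi reaches it.
; Overlap of its PickUpBoundary by a BP_Taxi adds a WBP_PassengerInteraction widget to the viewport, which a named timer removes seconds later.
; A separate SpawnPickUpPointEvent, not called within this Blueprint, spawns a BP_PickUpPoint in front of the passenger.
; The SpawnStartPointEvent dispatcher bind and call are disconnected leftovers.
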(event OnComponentBeginOverlap(PickUpBoundary)
  (params (OverlappedComponent :type Primitive%20Component%20Object%20Reference) (OtherActor :type Actor%20Object%20Reference) (OtherComp :type Primitive%20Component%20Object%20Reference) (OtherBodyIndex :type Integer) (bFromSweep :type Boolean) (SweepResult :type Hit%20Result%20Structure%20%28by%20ref%29))
  (bind _asbp_taxi (Utilities|Casting|CastToBP_Taxi OtherActor))
  (if (Utilities|IsValid _asbp_taxi)
    ;[1 1 1] 위젯을 화면 정중앙에 띄우기
    (bind _returnvalue (UserInterface|CreateWidget "/Game/JiYoung/Widget_jy/WBP_PassengerInteraction.WBP_PassengerInteraction_C" (Game|GetPlayerController (Variables|Default|GetPlayer%20Index))))
    (bind _output_get (Variables|Default|SetPassengerWidgetInstance _returnvalue))
    (UserInterface|Viewport|AddtoViewport _output_get 0)
    ;[1 1 1] n초 후 위젯 사라짐
    (Utilities|Time|SetTimerbyFunctionName 0 "RemoveWidget" 5.0)))

(event Custom|SpawnPickUpPointEvent
  (Game|SpawnActorfromClass "/Game/JiYoung/Blueprints_jy/BP_PickUpPoint.BP_PickUpPoint_C" (Math|Transform|MakeTransform (+ (* (Transformation|GetActorForwardVector) 5e+02) (Transformation|GetActorLocation))) "Undefined" "MultiplyWithRoot" 0 0))

(event EventBeginPlay
  (Variables|Default|SetPassengerRef 0))

(fn ConstructionScript)

(fn RemoveWidget
  (bind _passengerwidgetinstance (Variables|Default|GetPassengerWidgetInstance))
  (if (Utilities|IsValid _passengerwidgetinstance)
    (Widget|RemovefromParent _passengerwidgetinstance)))