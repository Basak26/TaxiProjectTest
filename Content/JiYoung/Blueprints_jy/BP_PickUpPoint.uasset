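; BP_PickUpPoint is a taxi pickup zone that hands off to a drop-off destination.
; BeginPlay hides the marker on every BP_DropOffPoint.
; When BP_Taxi overlaps Box_PickUp, the pickup marker hides, then after a short delay the referenced Passenger's mesh hides and DropOffPointRef's marker appears.
; Boarding is purely visibility toggling; the Passenger lookup is disconnected, and nothing here assigns DropOffPointRef.
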(event OnComponentBeginOverlap(Box_PickUp)
  (params (OverlappedComponent :type Primitive%20Component%20Object%20Reference) (OtherActor :type Actor%20Object%20Reference) (OtherComp :type Primitive%20Component%20Object%20Reference) (OtherBodyIndex :type Integer) (bFromSweep :type Boolean) (SweepResult :type Hit%20Result%20Structure%20%28by%20ref%29))
  (bind _asbp_taxi (Utilities|Casting|CastToBP_Taxi OtherActor))
  (if (Utilities|IsValid _asbp_taxi)
    ;[1 1 1] 승차 구역 도달 시 startpoint 사라짐
    (Rendering|SetVisibility (Variables|Default|GetPickUpPoint) false false)
    ;[1 1 1] n초 후에 손님 탑승(모습 사라짐)
    (Utilities|FlowControl|Delay 3.0)
    (Rendering|SetVisibility (Variables|/Game/JiYoung/Blueprints_jy/BP_Passenger.BP_Passenger_C|GetSkeletalMesh (Variables|Default|GetPassenger)) false false)
    ;[1 1 1] 동시에 하차 목적지 활성화(눈에 보임)
    (Rendering|SetVisibility (Variables|/Game/JiYoung/Blueprints_jy/BP_DropOffPoint.BP_DropOffPoint_C|GetDropOffPoint (Variables|Default|GetDropOffPointRef)) true false)))

(event Collision|EventActorBeginOverlap
  (params (OtherActor :type Actor%20Object%20Reference)))

(event EventTick
  (params (DeltaSeconds :type Float%20%28single-precision%29)))

(event EventBeginPlay
  ;[1 1 1] 게임시작할 때 하차 목적지 안 보이게 설정
  (bind _outactors (Actor|GetAllActorsOfClass "/Game/JiYoung/Blueprints_jy/BP_DropOffPoint.BP_DropOffPoint_C"))
  (for _array_element _outactors
    (Rendering|SetVisibility (Variables|/Game/JiYoung/Blueprints_jy/BP_DropOffPoint.BP_DropOffPoint_C|GetDropOffPoint _array_element) false false)))

(fn ConstructionScript)